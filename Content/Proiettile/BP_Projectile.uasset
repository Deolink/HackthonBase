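; BP_Projectile is a projectile actor that damages the actor it hits and then destroys itself.
; When its ProjectileMovement component stops, it passes the hit actor to DamageHit.
; DamageHit looks for a BPC_PlayerStatComponent on that actor and, if one exists, subtracts Danno through RimuoviVita.
; The projectile is destroyed whether or not that component is found.
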(event OnProjectileStop(ProjectileMovement)
  (params (ImpactResult :type Hit%20Result%20Structure%20%28by%20ref%29))
  (CallFunction|DamageHit (.hitactor ImpactResult)))

(event EventBeginPlay)

(event Collision|EventActorBeginOverlap
  (params (OtherActor :type Actor%20Object%20Reference)))

(event EventTick
  (params (DeltaSeconds :type Float%20%28single-precision%29)))

(fn ConstructionScript)

(fn DamageHit
  (params (Actor :type Actor%20Object%20Reference))
  (bind _output_get (LocalVariables|SetStatComponent (Actor|GetComponentbyClass Actor "/Game/Components/BPC_PlayerStatComponent.BPC_PlayerStatComponent_C")))
  (Utilities|IsValid _output_get
    (:Is%20Valid
      (Default|RimuoviVita (LocalVariables|GetStatComponent) (Variables|Default|GetDanno)))
    (:Is%20Not%20Valid
      _))
  (Actor|DestroyActor))
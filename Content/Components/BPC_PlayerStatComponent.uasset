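; Player stat component that tracks health (Vita), energy (Energia) and experience (Esperienza).
; Health functions add or subtract directly, while both energy functions have unconnected logic and change nothing.
; Adding experience fires an event dispatcher, bound on BeginPlay, that asks the owner's BPC_PowerUp whether double jump applies.
; If it does, the owning Character's max jump count becomes two.
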(event Custom|ModificaEsperienza
  (bind _canjump (Default|DoubleJump (Actor|GetComponentbyClass (Components|GetOwner) "/Game/Components/BPC_PowerUp.BPC_PowerUp_C") (Variables|Default|GetEsperienzaGiocatore)))
  (if _canjump
    (bind _ascharacter (Utilities|Casting|CastToCharacter (Components|GetOwner)))
    (Variables|/Script/Engine.Character|SetJumpMaxCount _ascharacter 2)))

(event EventBeginPlay
  (EventDispatchers|BindEventtoEsperienzaListener (delegate Custom|ModificaEsperienza)))

(fn RimuoviVita
  (params (danno :type Integer))
  (Variables|Default|SetVitaGiocatore (- (Variables|Default|GetVitaGiocatore) danno)))

(fn AggiungiVita
  (params (vita :type Integer))
  (Variables|Default|SetVitaGiocatore (+ (Variables|Default|GetVitaGiocatore) vita)))

(fn AggiungiEnergia
  (params (energia :type Integer)))

(fn RimuoviEnergia
  (params (energia :type Integer)))

(fn AggiungiEsperienza
  (params (esperienza :type Integer))
  (Variables|Default|SetEsperienzaGiocatore (+ esperienza (Variables|Default|GetEsperienzaGiocatore)))
  (Default|CallEsperienzaListener)
  (return (Variables|Default|GetEsperienzaGiocatore)))
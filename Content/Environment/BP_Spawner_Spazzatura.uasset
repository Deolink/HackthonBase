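; BP_Spawner_Spazzatura is a spawner that launches a "spazzatura" (trash) actor when the 1 key is pressed.
; It spawns the actor at its Arrow component, scaled down, then applies a velocity-change impulse to SMBody along the arrow's forward vector, scaled by ImpulseForce.
; An alternative function spawns above the spawner's own location but is not called in this graph.
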(event EventBeginPlay)

(event Collision|EventActorBeginOverlap
  (params (OtherActor :type Actor%20Object%20Reference)))

(event EventTick
  (params (DeltaSeconds :type Float%20%28single-precision%29)))

(event Input|KeyboardEvents|1
  (params (Key :type Key%20Structure))
  (:Pressed
    (bind _returnvalue (CallFunction|SpawnSpazzaturaatLocation))
    (Physics|AddImpulse (Variables|Default|GetSM_Body _returnvalue) (CallFunction|GetImpulseDirection) "None" true)))

(fn ConstructionScript)

(fn GetSpawnTransform
  (bind _returnvalue (Transformation|GetActorLocation))
  (bind (_x _y _z) (Math|Vector|BreakVector _returnvalue))
  (return (Math|Transform|MakeTransform (Math|Vector|MakeVector _x _y (+ _z 5e+02)))))

(fn SpawnSpazzaturaatActorLocation
  (Game|SpawnActorfromClass 0 (CallFunction|GetSpawnTransform) "Undefined" 0 0))

(fn SpawnSpazzaturaatLocation
  (bind _returnvalue (Game|SpawnActorfromClass 0 (Math|Transform|MakeTransform (Transformation|GetWorldLocation (Variables|Default|GetArrow)) "0, 0, 0" "0.200000,0.200000,0.200000") "Undefined" 0 0))
  (return _returnvalue))

(fn GetImpulseDirection
  (return (* (Math|Vector|GetForwardVector (Variables|Default|GetArrow)) (Math|Float|MakeLiteralFloat (Variables|Default|GetImpulse%20Force%20)))))